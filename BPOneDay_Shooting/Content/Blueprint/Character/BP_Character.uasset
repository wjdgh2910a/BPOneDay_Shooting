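; BP_Character is a character Blueprint with shared movement helpers and rifle firing.
; Helpers yaw the actor toward a target location with a rotation offset, return velocity in local space, and report whether it is moving.
; Fire is gated by CanFire: it plays the fire montage, triggers the BP_Rifle held in a ChildActor component, and starts a cooldown timer whose OnFire callback re-enables firing.
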(event EventBeginPlay)

(event Collision|EventActorBeginOverlap
  (params (OtherActor :type Actor%20Object%20Reference)))

(event EventTick
  (params (DeltaSeconds :type Float%20%28single-precision%29)))

(fn ConstructionScript)

(fn LooktoLocation
  (params (TargetLocation :type Vector))
  (Transformation|SetActorRotation (Math|Rotator|MakeRotator 0.0 0.0 (- (.yaw (Math|Rotator|FindLookatRotation (Transformation|GetActorLocation) TargetLocation)) (Variables|Default|GetRotationOffset)))))

(fn GetMoveVelocity
  (return (Math|Transform|InverseTransformDirection (Transformation|GetActorTransform) (Variables|/Script/Engine.MovementComponent|GetVelocity (Variables|Character|GetCharacterMovement)))))

(fn IsMove
  (return (!= (Math|Vector|VectorLength (Variables|/Script/Engine.MovementComponent|GetVelocity (Variables|Character|GetCharacterMovement))) 0.0)))

(fn Fire
  (if (Variables|Default|GetCanFire)
    (Utilities|FlowControl|Sequence
      (:then_0
        (Variables|Default|SetCanFire false)
        (Animation|Montage|MontagePlay (Components|SkeletalMesh|GetAnimInstance (Variables|Character|GetMesh)) "/Game/Blueprint/Character/Animation/AM_Fire.AM_Fire" 1.0 "MontageLength" 0.0 true)
        (Utilities|Time|SetTimerbyFunctionName 0 "OnFire" (Variables|Default|GetFireCoolTime)))
      (:then_1
        (bind _asbp_rifle (Utilities|Casting|CastToBP_Rifle (Variables|/Script/Engine.ChildActorComponent|GetChildActor (Variables|Default|GetChildActor))))
        (Default|Fire _asbp_rifle)))))

(fn OnFire
  (Variables|Default|SetCanFire true))