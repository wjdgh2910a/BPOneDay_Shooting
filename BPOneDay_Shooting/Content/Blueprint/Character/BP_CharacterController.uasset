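; BP_CharacterController is a player controller for a top-down-style character that moves by input and aims at the mouse cursor.
; On BeginPlay it adds the IMC_Character Enhanced Input context and shows the cursor.
; Each tick it traces under the cursor on the Visibility channel and passes the hit location to BP_Character's LookToLocation.
; IA_Move adds world-axis movement to the pawn, and IA_Attack calls Fire on the character.
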(event Input|EnhancedActionEvents|EnhancedInputActionIA_Move
  (params (ActionValue :type Vector%202D%20Structure) (ElapsedSeconds :type Float%20%28double-precision%29) (TriggeredSeconds :type Float%20%28double-precision%29) (InputAction :type Input%20Action%20Object%20Reference :default "/Game/Blueprint/Character/Input/IA_Move.IA_Move"))
  (Pawn|Input|AddMovementInput (Pawn|GetControlledPawn) (Math|Vector|MakeVector (.x ActionValue) (.y ActionValue) 0.0) 1.0 false))

(event Input|EnhancedActionEvents|EnhancedInputActionIA_Attack
  (params (ActionValue :type Boolean) (ElapsedSeconds :type Float%20%28double-precision%29) (TriggeredSeconds :type Float%20%28double-precision%29) (InputAction :type Input%20Action%20Object%20Reference :default "/Game/Blueprint/Character/Input/IA_Attack.IA_Attack"))
  (bind _asbp_character (Utilities|Casting|CastToBP_Character (Pawn|GetControlledPawn)))
  (Default|Fire _asbp_character))

(event EventBeginPlay
  (bind _self self)
  (bind _returnvalue (PlayerController|LocalPlayerSubsystems|GetEnhancedInputLocalPlayerSubsystem _self))
  (Utilities|IsValid _returnvalue
    (:Is%20Valid
      (Input|AddMappingContext _returnvalue "/Game/Blueprint/Character/Input/IMC_Character.IMC_Character" 0 "(bIgnoreAllPressedKeysUntilRelease=True,bForceImmediately=False,bNotifyUserSettings=False)")
      (Variables|Default|SetbShowMouseCursor true))))

(event EventTick
  (params (DeltaSeconds :type Float%20%28single-precision%29))
  (bind (_hitresult _returnvalue) (Game|Player|GetHitResultUnderCursorbyChannel "TraceTypeQuery1" false))
  (bind _asbp_character (Utilities|Casting|CastToBP_Character (Pawn|GetControlledPawn)))
  (if _returnvalue
    (bind _output_get (Variables|Default|SetMousePosition (.location _hitresult)))
    (Default|LooktoLocation _asbp_character _output_get)))

(fn ConstructionScript)