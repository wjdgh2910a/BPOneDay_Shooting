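; BP_Rifle is a hitscan rifle weapon that damages zombies.
; Fire spawns an effect at the FirePoint, then line traces on Visibility with debug drawing and calls Hit on any BP_Zombi it strikes.
; The trace end comes from GetFireEndLocation, which extends a fixed range from the FirePoint toward the MousePosition stored on the player's BP_CharacterController.
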(event EventBeginPlay)

(event Collision|EventActorBeginOverlap
  (params (OtherActor :type Actor%20Object%20Reference)))

(event EventTick
  (params (DeltaSeconds :type Float%20%28single-precision%29)))

(fn ConstructionScript)

(fn Fire
  (bind _endlocation (CallFunction|GetFireEndLocation))
  (Niagara|SpawnSystematLocation "/Game/Effects/Particles/Weapons/Emitters/FireEffect.FireEffect" (Transformation|GetWorldLocation (Variables|Default|GetFirePoint)) "-90.000000,0.000000,0.000000")
  (bind (_outhit _returnvalue) (Collision|LineTraceByChannel (Transformation|GetWorldLocation (Variables|Default|GetFirePoint)) (Math|Vector|MakeVector (.x _endlocation) (.y _endlocation) (.z _endlocation)) "TraceTypeQuery1" false 0 "ForDuration" true "(R=1.000000,G=0.000000,B=0.000000,A=1.000000)" "(R=0.000000,G=1.000000,B=0.000000,A=1.000000)" 1.0))
  (if _returnvalue
    (bind _asbp_zombi (Utilities|Casting|CastToBP_Zombi (.hitactor _outhit)))
    (Default|Hit _asbp_zombi)))

(fn GetFireEndLocation
  (bind _asbp_character_controller (Utilities|Casting|CastToBP_CharacterController (Game|GetPlayerController 0)))
  (return (+ (* (Math|Vector|Normalize (- (Variables|/Game/Blueprint/Character/BP_CharacterController.BP_CharacterController_C|GetMousePosition _asbp_character_controller) (Transformation|GetWorldLocation (Variables|Default|GetFirePoint)))) 1e+03) (Transformation|GetWorldLocation (Variables|Default|GetFirePoint)))))