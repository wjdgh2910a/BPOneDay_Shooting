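; Zombie enemy pawn that chases the player and can be killed by repeated hits.
; It caches the player character on BeginPlay, then feeds movement input straight toward it every Tick, with no pathfinding.
; Hit decrements LifeCount and destroys the actor when it runs out.
; Otherwise, it nearly freezes the zombie through CustomTimeDilation as a hit-stun, and a HitTime timer calls RecoveryHit to restore normal speed.
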(event EventBeginPlay
  (Variables|Default|SetTarget (Game|GetPlayerCharacter 0)))

(event Collision|EventActorBeginOverlap
  (params (OtherActor :type Actor%20Object%20Reference)))

(event EventTick
  (params (DeltaSeconds :type Float%20%28single-precision%29))
  (Pawn|Input|AddMovementInput (Math|Vector|Normalize (- (Transformation|GetActorLocation (Variables|Default|GetTarget)) (Transformation|GetActorLocation))) 1.0 false))

(fn ConstructionScript)

(fn Hit
  (bind _result (Math|Integer|DecrementInt (Variables|Default|GetLifeCount))
    (:%20%20
      (if (<= _result 0)
        (Actor|DestroyActor)
        (else
          (Variables|Default|SetCustomTimeDilation 0.0001)
          (Utilities|Time|SetTimerbyFunctionName 0 "RecoveryHit" (Variables|Default|GetHitTime)))))))

(fn RecoveryHit
  (Variables|Default|SetCustomTimeDilation 1.0))